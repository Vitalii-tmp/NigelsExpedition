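; MovebleColumn is a level column that the Nigel character can push.
; Overlap events on the X-axis and Y-axis collision components cast to Nigel, enable physics simulation on the Column and set Nigel's IsPushing flag.
; Leaving either zone clears IsPushing but sets physics simulation to true again, so nothing here switches it back off.
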(event `self.Y Axis Collision.OnComponentBeginOverlap`
  (params (OverlappedComponent :type "PrimitiveComponent Object Reference") (OtherActor :type "Actor Object Reference") (OtherComp :type "PrimitiveComponent Object Reference") (OtherBodyIndex :type Integer) (bFromSweep :type Boolean) (SweepResult :type "HitResult Structure (by ref)"))
  ;[1 1 1] Y Axis Collision
  (bind _asnigel (cast `Nigel` OtherActor))
  (`PrimitiveComponent.SetSimulatePhysics` (`self.Column`) true)
  (set `Nigel.IsPushing` true _asnigel))

(event `self.Y Axis Collision.OnComponentEndOverlap`
  (params (OverlappedComponent :type "PrimitiveComponent Object Reference") (OtherActor :type "Actor Object Reference") (OtherComp :type "PrimitiveComponent Object Reference") (OtherBodyIndex :type Integer))
  ;[1 1 1] Y Axis Collision
  (bind _asnigel (cast `Nigel` OtherActor))
  (`PrimitiveComponent.SetSimulatePhysics` (`self.Column`) true)
  (set `Nigel.IsPushing` false _asnigel))

(event `self.X Axis Collision.OnComponentBeginOverlap`
  (params (OverlappedComponent :type "PrimitiveComponent Object Reference") (OtherActor :type "Actor Object Reference") (OtherComp :type "PrimitiveComponent Object Reference") (OtherBodyIndex :type Integer) (bFromSweep :type Boolean) (SweepResult :type "HitResult Structure (by ref)"))
  ;[1 1 1] Y Axis Collision
  (bind _asnigel (cast `Nigel` OtherActor))
  (`PrimitiveComponent.SetSimulatePhysics` (`self.Column`) true)
  (set `Nigel.IsPushing` true _asnigel))

(event `self.X Axis Collision.OnComponentEndOverlap`
  (params (OverlappedComponent :type "PrimitiveComponent Object Reference") (OtherActor :type "Actor Object Reference") (OtherComp :type "PrimitiveComponent Object Reference") (OtherBodyIndex :type Integer))
  ;[1 1 1] Y Axis Collision
  (bind _asnigel (cast `Nigel` OtherActor))
  (`PrimitiveComponent.SetSimulatePhysics` (`self.Column`) true)
  (set `Nigel.IsPushing` false _asnigel))

(fn `UserConstructionScript`)